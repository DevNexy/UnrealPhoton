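; Card is an actor Blueprint for a colored, labeled card that other code places by X/Y coordinates.
; The construction script creates a dynamic material instance on the mesh, which setColor tints, optionally attaching a border decal to mark the local actor.
; Other events move the card in 100-unit steps on the ground plane, set its text, and scale that text uniformly by grid size.
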(event Custom|move
  (params (x :type Integer) (y :type Integer))
  (Transformation|SetActorTransform (Math|Transform|MakeTransform (Math|Vector|MakeVector (* x 1e+02) (* y 1e+02) 0.0))))

(event Custom|setColor
  (params (col :type Linear%20Color%20Structure) (border :type Boolean))
  (Rendering|Material|SetVectorParameterValue (Variables|Default|GetDynamicMaterial) "The Color" col :!class /Script/Engine.MaterialInstanceDynamic)
  ;[1 1 1] Draw border for local actor
  (if border
    (Class|GameplayStatics|SpawnDecalAttached "/Game/Materials/CardBorderDecal.CardBorderDecal" "50.000000,50.000000,50.000000" (Variables|Default|GetStaticMesh1) "" "0,0.000000, 0" "90.000000, 0, 0" "KeepRelativeOffset" 0.0)))

(event Custom|UpdateTextSize
  (params (gridSize :type Integer))
  (bind _returnvalue (Math|Conversions|ToFloat(Integer) gridSize))
  (Transformation|SetRelativeScale3D (Variables|Default|GetTextRender1) (Math|Vector|MakeVector _returnvalue _returnvalue _returnvalue)))

(event Custom|SetText
  (params (text :type String))
  (Rendering|Components|TextRender|SetText (Variables|Default|GetTextRender1) (Utilities|Text|ToText(String) text)))

(fn ConstructionScript
  (bind _returnvalue (Rendering|Material|CreateDynamicMaterialInstance (Variables|Default|GetStaticMesh1) 0 "/Game/Materials/card.Card" :!class /Script/Engine.PrimitiveComponent))
  (Variables|Default|SetDynamicMaterial _returnvalue))