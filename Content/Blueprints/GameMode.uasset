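; Game mode that sets up Photon chat and voice communication and shows the main menu when play begins.
; If the first player's pawn is a BP_Pawn_Player, it spawns Photon chat and voice client actors, stores references and connects both with a hardcoded name.
; It then creates the WB_MainMenu widget, keeps a reference and adds it to the viewport.
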(event Custom|SpawnActor_Photon_All
  (bind _returnvalue (Math|Transform|MakeTransform "0, 0, 0"))
  (Utilities|Casting|CastToBP_Pawn_Player (Game|Player|GetPlayerPawn 0))
  (bind _returnvalue_2 (Game|SpawnActorfromClass "/Game/Blueprints/PhotonChatClient.PhotonChatClient_C" _returnvalue "AlwaysSpawn" "MultiplyWithRoot" 0 0))
  (bind _output_get (Variables|Default|SetPhotonChat _returnvalue_2))
  (bind _returnvalue_3 (Game|SpawnActorfromClass "/Game/Blueprints/PhotonVoiceClient.PhotonVoiceClient_C" _returnvalue "AlwaysSpawn" "MultiplyWithRoot" 0 0))
  (bind _output_get_2 (Variables|Default|SetPhotonVoice _returnvalue_3))
  (Class|ActorPhotonVoice|Connect _output_get_2 "jiwon")
  (Class|ActorPhotonChat|ConnectChat _output_get "jiwon"))

(event Custom|CreateMainMenu
  (Development|PrintString "// Widget :: Main Menu Create")
  (bind _returnvalue (UserInterface|CreateWidget "/Game/Blueprints/WB_MainMenu.WB_MainMenu_C"))
  (bind _output_get (Variables|Default|SetWB_MainMenu _returnvalue))
  (UserInterface|Viewport|AddtoViewport _output_get 0))

(event EventBeginPlay
  (CallFunction|SpawnActorPhotonAll)
  (CallFunction|CreateMainMenu))

(fn ConstructionScript)