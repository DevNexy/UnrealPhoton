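; Actor Blueprint for a Photon chat client that shows chat messages in the main menu's chat room widget.
; Incoming-message events reach that widget through the GameMode's main menu reference and add each message as a Public channel slot.
; Live messages show the sender's name, while a received batch of past messages is looped through and labeled "previous".
; The connect-complete event is an empty stub.
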(event EventBeginPlay)

(event Collision|EventActorBeginOverlap
  (params (OtherActor :type Actor%20Object%20Reference)))

(event EventTick
  (params (DeltaSeconds :type Float%20%28single-precision%29)))

(event EventBlueprintConnectComplete)

(event EventBlueprintGetMessageEvent
  (params (ChannelName :type String) (Sender :type String) (Message :type String))
  (bind _asgame_mode (Utilities|Casting|CastToGameMode (Game|GetGameMode)))
  (Utilities|IsValid (Variables|/Game/Blueprints/GameMode.GameMode_C|GetWB_MainMenu _asgame_mode)
    (:Is%20Valid
      (Default|AddChatMessageSlot (Variables|/Game/Blueprints/WB_MainMenu.WB_MainMenu_C|GetWB_ChatingRoom (Variables|/Game/Blueprints/GameMode.GameMode_C|GetWB_MainMenu _asgame_mode)) "Public" Sender Message))))

(event EventBluerprintReceivedMessageEvent
  (params (Messages :type Array%20of%20Strings))
  ;[1 1 1] 과거 받은 메세지 출력
  (bind _asgame_mode (Utilities|Casting|CastToGameMode (Game|GetGameMode)))
  (Utilities|IsValid (Variables|/Game/Blueprints/GameMode.GameMode_C|GetWB_MainMenu _asgame_mode)
    (:Is%20Valid
      (for _array_element Messages
        (Default|AddChatMessageSlot (Variables|/Game/Blueprints/WB_MainMenu.WB_MainMenu_C|GetWB_ChatingRoom (Variables|/Game/Blueprints/GameMode.GameMode_C|GetWB_MainMenu _asgame_mode)) "Public" "previous" _array_element)))))

(fn ConstructionScript)