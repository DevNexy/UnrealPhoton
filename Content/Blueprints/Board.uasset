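; Board actor that serves as a resizable grid floor with a toggleable checker pattern, apparently for a Photon multiplayer game.
; The construction script creates a dynamic material; Setup scales the actor and grid texture to the grid size, and UpdateCheckerVisibility toggles the checker parameter.
; Unconnected event-graph logic would project the dragged mouse onto the Z=0 plane and send the floored cell to Photonclient as the local player position.
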(event Input|MouseEvents|MouseX
  (params (AxisValue :type Float%20%28single-precision%29))
  ;[1 1 1] Moving player by mouse
)

(event Input|MouseEvents|MouseY
  (params (AxisValue :type Float%20%28single-precision%29))
  ;[1 1 1] Moving player by mouse
)

(event Input|MouseEvents|LeftMouseButton
  (params (Key :type Key%20Structure :default "None"))
  ;[1 1 1] Moving player by mouse
)

(fn ConstructionScript
  (bind _returnvalue (Rendering|Material|CreateDynamicMaterialInstance (Variables|Default|GetStaticMesh1) 0 "/Game/Materials/board.board" "None" :!class /Script/Engine.PrimitiveComponent))
  (Variables|Default|SetDynamicMaterial _returnvalue))

(fn Setup
  (params (gridSize :type Integer))
  (bind _returnvalue (Math|Conversions|ToFloat(Integer) gridSize))
  ;[1 1 1] Called on start and when board size changed
  (Transformation|SetActorRelativeScale3D (Math|Vector|MakeVector _returnvalue _returnvalue 1.0))
  ;;[1 1 1] Scaling grid texture uv to match grid size
  (Rendering|Material|SetScalarParameterValue (Variables|Default|GetDynamicMaterial) "Scale" (Math|Conversions|ToFloat(Integer) gridSize) :!class /Script/Engine.MaterialInstanceDynamic))

(fn UpdateCheckerVisibility
  (params (visible :type Boolean))
  (Rendering|Material|SetScalarParameterValue (Variables|Default|GetDynamicMaterial) "showChecker" (Math|Conversions|ToFloat(Boolean) visible) :!class /Script/Engine.MaterialInstanceDynamic))